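; Inventory component that stores items as stacked entries and lets the Kwang player character use utility items.
; On BeginPlay it caches the player and spawns an A_Item_Recording actor at a set location.
; Adding stacks items by ID, while removal matches the item itself; UseItem adds a utility item's Vie to HP, unclamped, then removes one.
; A helper returns a forward offset from the owner, rotated around Z by an input multiplier.
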(event `self.ReceiveBeginPlay`
  (`|ExecutionSequence`
    (:`then_0`
      (bind _askwang_player_character (cast `/Game/Rayane/Player/KwangPlayerCharacter` (`GameplayStatics.GetPlayerCharacter` 0)))
      (set `self.Player REF` _askwang_player_character))
    (:`then_1`
      (bind _returnvalue (`|SpawnActorFromClass` "/Game/Chris/Inventaire/Prévisu/A_Item_Recording.A_Item_Recording_C" (`KismetMathLibrary.MakeTransform` (`self.RecordingActorLocation`)) "AlwaysSpawn" "MultiplyWithRoot" null null))
      (set `self.RecordingActorRef` _returnvalue))))

(event `/Game/Chris/Inventaire/I_Inventaire.UseItem`
  (params (Item :type "/Game/Chris/Inventaire/Item_Object/ObjClass_ItemBase Object Reference"))
  (bind _player_ref (`self.Player REF`))
  (bind ((`MaxHP_37_70A61075474F3DD841D7FD928659E63E` _maxhp) (`MaxMana_38_4BFFD65A4A16722440BB96986D4F9384` _maxmana) (`Mana_14_39BB52B346A448CDE04938905026B1E6` _mana) (`Strength_21_D86C58A44783F1EA40804B8FE5757D63` _strength) (`Intelligence_19_F8F5ED184CDF5476728DE5B1209159E9` _intelligence) (`Dexterity_18_AA4606084CC8F3373A7BC4ADAE94EB92` _dexterity) (`Speed_17_1DE2F7E1415EF3993454C79098D25AD4` _speed) (`Evasion_8_852242334E3EAEB2805CC59F97E5F01A` _evasion) (`Defence_26_2379EDEC4A095053D00EADAD75F2A5AA` _defence) (`XP_23_B01B204E49499B6BB2B3A9A53C4E89BA` _xp) (`Level_25_7751461748A62D8799E73EA60251160D` _level) (`QuestName_31_A722A0274A919186AADB03A259F93F7D` _questname) (`QuestText_32_E2FC44534B98D362B51DED98CFD2213F` _questtext) (`IsDead_41_FB479626496BAE97E6CF578ED555126A` _isdead)) (break `/Game/Rayane/Structures/STR_Stats` (`/Game/Rayane/Player/KwangPlayerCharacter.Stats` _player_ref)))
  (set `self.Item REF` Item)
  (`|ExecutionSequence`
    (:`then_0`
      (bind _asobj_class_item_utilitaires (cast `/Game/Chris/Inventaire/Item_Object/ObjClass_ItemUtilitaires` (`self.Item REF`))
        (:`then`
          (set `/Game/Rayane/Player/KwangPlayerCharacter.Stats` (make `/Game/Rayane/Structures/STR_Stats` _maxhp (`KismetMathLibrary.FTrunc` (+ (`/Game/Chris/Inventaire/Item_Object/ObjClass_ItemUtilitaires.Vie` _asobj_class_item_utilitaires) (`.HP_12_6A8A12A94A00EEB9E5672A86E3E90C43` (break `/Game/Rayane/Structures/STR_Stats` (`/Game/Rayane/Player/KwangPlayerCharacter.Stats` (`self.Player REF`)))))) _maxmana _mana _strength _intelligence _dexterity _speed _evasion _defence _xp _level _questname _questtext _isdead) _player_ref)
          (`self.Remove from inventory` (`self.Item REF`)))
        (:`CastFailed`
          (`KismetSystemLibrary.PrintString` "Cast Failed"))))))

(fn `Add to inventory`
  (params (`Item to add` :type "/Game/Chris/Inventaire/Item_Object/ObjClass_ItemBase Object Reference"))
  (locals (index :type Integer) (`found same item` :type Boolean))
  (bind (_nb _item) (break `/Game/Chris/Inventaire/Struct_ItemInventory` (`|GetArrayItem` (`self.inventory item`) (`local.index`))))
  (set `self.Item To Add` `Item to add`)
  (for (_array_element _array_index) (`self.inventory item`)
    (if (`KismetTextLibrary.EqualEqual_TextText` (`/Game/Chris/Inventaire/Item_Object/ObjClass_ItemBase.ID` (`self.Item To Add`)) (`/Game/Chris/Inventaire/Item_Object/ObjClass_ItemBase.ID` (`.Item_6_163A80E4484456080339499EE072BFD4` (break `/Game/Chris/Inventaire/Struct_ItemInventory` _array_element))))
      (set `local.index` _array_index)
      (set `local.found same item` true)
      (break)))
  (if (`local.found same item`)
    (`KismetArrayLibrary.Array_Set` (`self.inventory item`) (`local.index`) (make `/Game/Chris/Inventaire/Struct_ItemInventory` (+ _nb 1) _item))
    (else
      (`KismetArrayLibrary.Array_Add` (`self.inventory item`) (make `/Game/Chris/Inventaire/Struct_ItemInventory` 1 (`self.Item To Add`))))))

(fn `GetRotatedFromPlayerLocation`
  (params (`Get Rotated From Player Location` :type Integer))
  (returns (Location :type "Vector Structure"))
  (return (`KismetMathLibrary.RotateAngleAxis` (* (`Actor.GetActorForwardVector` (`self.GetOwner`)) 250.0) (* `Get Rotated From Player Location` 20.0) (0.0 0.0 1.0))))

(fn `Remove from inventory`
  (params (`item to remove` :type "/Game/Chris/Inventaire/Item_Object/ObjClass_ItemBase Object Reference"))
  (locals (index :type Integer))
  (bind (_nb _item) (break `/Game/Chris/Inventaire/Struct_ItemInventory` (`|GetArrayItem` (`self.inventory item`) (`local.index`))))
  (for (_array_element _array_index) (`self.inventory item`)
    (if (== `item to remove` (`.Item_6_163A80E4484456080339499EE072BFD4` (break `/Game/Chris/Inventaire/Struct_ItemInventory` _array_element)))
      (set `local.index` _array_index)
      (break)))
  (if (> _nb 1)
    (`KismetArrayLibrary.Array_Set` (`self.inventory item`) (`local.index`) (make `/Game/Chris/Inventaire/Struct_ItemInventory` (- _nb 1) _item))
    (else
      (`KismetArrayLibrary.Array_Remove` (`self.inventory item`) (`local.index`)))))