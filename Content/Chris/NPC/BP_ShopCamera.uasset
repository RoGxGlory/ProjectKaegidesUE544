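; BP_ShopCamera is a shop camera that identifies its role (main, left side or right side) to the shopkeeper NPC system.
; On BeginPlay it finds BP_NPC_Shopkeeper and binds to that actor's SetCamera dispatcher.
; When that fires, its role booleans choose which validate-camera dispatcher broadcasts a reference to itself.
; If no role is set, it prints a warning.
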(event `self.ReceiveBeginPlay`
  (bind _returnvalue (`GameplayStatics.GetActorOfClass` "/Game/Chris/NPC/BP_NPC_Shopkeeper.BP_NPC_Shopkeeper_C"))
  (bind _output_get (set `self.Shopkeeper` _returnvalue))
  (add `/Game/Chris/NPC/BP_NPC_Shopkeeper.Set Camera` _output_get (delegate `Set Camera_Event`)))

(event `Set Camera_Event`
  (if (`self.bIsShopCamera`)
    (`self.ValidateCamera` self)
    (elif (`self.bIsShopLeftSideCamera`)
      (`self.ValidateLeftSideCamera` self)
      (elif (`self.bIsShopRightSideCamera`)
        (`self.ValidateRightSideCamera` self)
        (else
          (`KismetSystemLibrary.PrintString` "Camera is not set" true true (struct :`R` 1.0 :`G` 0.013839 :`A` 1.0)))))))

(fn `UserConstructionScript`)