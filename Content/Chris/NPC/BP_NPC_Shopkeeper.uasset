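; Shopkeeper NPC that opens the shop when the player walks into its trigger.
; On BeginPlay it binds to every BP_ShopCamera's camera dispatchers, each storing into one Camera variable, then calls SetCamera and caches the KwangPlayerCharacter.
; On overlap, after a short delay, it blends the view to that camera, shows UI_Shop with UI-only input and cursor, and hides the player and fight HUD.
; Closing the shop is not handled here.
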(event `self.ReceiveBeginPlay`
  (bind _outactors (`GameplayStatics.GetAllActorsOfClass` "/Game/Chris/NPC/BP_ShopCamera.BP_ShopCamera_C"))
  (for _array_element _outactors
    (add `/Game/Chris/NPC/BP_ShopCamera.ValidateCamera` _array_element (delegate `ValidateCamera_Event`))
    (add `/Game/Chris/NPC/BP_ShopCamera.ValidateLeftSideCamera` _array_element (delegate `ValidateLeftSideCamera_Event`))
    (add `/Game/Chris/NPC/BP_ShopCamera.ValidateRightSideCamera` _array_element (delegate `ValidateRightSideCamera_Event`)))
  (bind _returnvalue (`GameplayStatics.GetActorOfClass` "/Game/Rayane/Player/KwangPlayerCharacter.KwangPlayerCharacter_C"))
  (set `self.Player` _returnvalue)
  (`self.Set Camera`))

(event `ValidateCamera_Event`
  (params (Camera :type "/Game/Chris/NPC/BP_ShopCamera Object Reference"))
  (set `self.Camera` Camera))

(event `ValidateLeftSideCamera_Event`
  (params (LeftSideCamera :type "/Game/Chris/NPC/BP_ShopCamera Object Reference"))
  (set `self.Camera` LeftSideCamera))

(event `ValidateRightSideCamera_Event`
  (params (RightSideCamera :type "/Game/Chris/NPC/BP_ShopCamera Object Reference"))
  (set `self.Camera` RightSideCamera))

(event `self.ShopTrigger.OnComponentBeginOverlap`
  (params (OverlappedComponent :type "PrimitiveComponent Object Reference") (OtherActor :type "Actor Object Reference") (OtherComp :type "PrimitiveComponent Object Reference") (OtherBodyIndex :type Integer) (bFromSweep :type Boolean) (SweepResult :type "HitResult Structure (by ref)"))
  (bind _returnvalue (`GameplayStatics.GetPlayerController` 0))
  (if (== OtherActor (`GameplayStatics.GetPlayerCharacter` 0))
    (`KismetSystemLibrary.Delay` 0.2)
    (`PlayerController.SetViewTargetWithBlend` (`GameplayStatics.GetPlayerController` 0) (`self.Camera`) 3.0 "VTBlend_Linear" 0.0 false)
    (bind _returnvalue_2 (`|CreateWidget` "/Game/Chris/UI/UI_Shop.UI_Shop_C"))
    (`UserWidget.AddToViewport` _returnvalue_2 0)
    (`WidgetBlueprintLibrary.SetInputMode_UIOnlyEx` _returnvalue _returnvalue_2 "LockOnCapture")
    (set `PlayerController.bShowMouseCursor` true _returnvalue)
    (`self.SetActorHiddenInGame` (`GameplayStatics.GetPlayerCharacter` 0) true)
    (`Widget.SetVisibility` (`/Game/Rayane/Player/KwangPlayerCharacter.FightHUD` (`self.Player`)) "Collapsed")
    (`KismetSystemLibrary.PrintString` "Hello")))

(fn `UserConstructionScript`)